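; BP_MotionController_Left is the left-hand VR motion controller actor, which lets the player show and hide a timer.
; Pressing face button 1 on the left controller runs a looping MultiGate that alternately unhides and hides the BPTimer child actor.
; BeginPlay, Tick and the construction script only call their parent implementations.
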(event EventTick
  (params (DeltaSeconds :type Float%20%28single-precision%29))
  (|CallParentFunction DeltaSeconds))

(event Collision|EventActorBeginOverlap
  (params (OtherActor :type Actor%20Object%20Reference)))

(event EventBeginPlay
  (|CallParentFunction))

(event Input|KeyboardEvents|MotionControllerLeftFaceButton1
  (params (Key :type Key%20Structure))
  (bind _bp_timer (Variables|Default|GetBP_Timer))
  (bind _childactor (Variables|/Script/Engine.ChildActorComponent|GetChildActor _bp_timer))
  (:Pressed
    (Utilities|FlowControl|MultiGate false true -1
      (:Out%200
        (Rendering|SetActorHiddenInGame _childactor false))
      (:Out%201
        (Rendering|SetActorHiddenInGame _childactor true)))))

(fn ConstructionScript
  (|CallParentFunction))