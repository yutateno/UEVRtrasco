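; BP_PlaySecondGun is a VR gun that BP_MotionController picks up and drops by attaching or detaching it, with physics simulation disabled at BeginPlay.
; While held, Tick polls the right gun-shot value and, past a trigger threshold, spawns BP_PlaySecondGunBall at the Sphere component's transform.
; A GunRush flag switches between spawning every tick and one shot per pull, using a DoOnce that resets when the trigger is released.
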(event EventBeginPlay
  (Physics|SetSimulatePhysics (Variables|Debug|GetStaticMeshComponent) false))

(event Collision|EventActorBeginOverlap
  (params (OtherActor :type Actor%20Object%20Reference)))

(event EventTick
  (params (DeltaSeconds :type Float%20%28single-precision%29))
  (if (Variables|Default|GetPickUpNow)
    (if (>= (Input|AxisValues|GetGunShotRight) 0.9)
      (if (Variables|Default|GetGunRush)
        _
        (else
          (Utilities|FlowControl|DoOnce false :!label _label
            (:Completed
              _))))
      (Game|SpawnActorfromClass "/Game/My/BP/Play/Second/BP_PlaySecondGunBall.BP_PlaySecondGunBall_C" (Transformation|GetWorldTransform (Variables|Default|GetSphere)) "AlwaysSpawn" 0 0)
      (else
        (goto _label Reset)))))

(event EventPickup
  (params (AttachTo :type Scene%20Component%20Object%20Reference))
  (Transformation|AttachComponentToComponent (VehicleSound|GetRootComponent) AttachTo "None" "KeepWorld" "KeepWorld" "KeepWorld" false)
  (Variables|Default|SetPickUpNow true))

(event EventDrop
  (Transformation|DetachFromActor "KeepWorld" "KeepWorld" "KeepWorld")
  (Variables|Default|SetPickUpNow false))

(fn ConstructionScript)