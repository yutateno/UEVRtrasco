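; BP_PlaySecondTarget is a target actor that slides back and forth along the X axis while changing to random colors.
; Tick flips the Hit flag at two hard-coded world X bounds and offsets the actor by a fixed, frame-rate-dependent step in that direction.
; A one-second Delay on Tick throttles the color change, which creates a new dynamic instance of M_Rainbow and randomizes its Param vector.
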(event EventBeginPlay)

(event Collision|EventActorBeginOverlap
  (params (OtherActor :type Actor%20Object%20Reference)))

(event EventTick
  (params (DeltaSeconds :type Float%20%28single-precision%29))
  (bind _returnvalue (Transformation|GetActorLocation))
  (if (< (.x _returnvalue) -8291.0)
    (Variables|Default|SetHit true))
  (if (> (.x _returnvalue) -6206.0)
    (Variables|Default|SetHit false))
  (if (Variables|Default|GetHit)
    (Transformation|AddActorWorldOffset (Math|Vector|MakeVector 1e+01 0.0 0.0))
    (else
      (Transformation|AddActorWorldOffset (Math|Vector|MakeVector -1e+01 0.0 0.0))))
  (Utilities|FlowControl|Delay 1.0)
  ;[1 1 1] 色変更処理
  (bind _returnvalue_2 (Rendering|Material|CreateDynamicMaterialInstance (Variables|Default|GetStaticMesh) 0 "/Game/My/Material/M_Rainbow.M_Rainbow" "None" :!class /Script/Engine.PrimitiveComponent))
  (Rendering|Material|SetVectorParameterValue _returnvalue_2 "Param" (Math|Color|MakeColor (Math|Random|RandomFloat) (Math|Random|RandomFloat) (Math|Random|RandomFloat)) :!class /Script/Engine.MaterialInstanceDynamic))

(fn ConstructionScript)