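; BP_PlaySecondGunBall is a gun projectile that destroys itself after seven seconds.
; On BeginPlay it reads BP_PlaySecondGunBallProcess flags to optionally randomize its color and enable one of eight movement components covering gravity, homing and turn combinations, or none.
; Turn adds a one-time, time-based sine/cosine velocity offset.
; Homing uses a component added to each BP_PlaySecondTarget, the last winning, with acceleration sign set by relative X position.
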(event EventBeginPlay
  (bind _returnvalue (Utilities|Time|GetTimeSeconds))
  (bind _returnvalue_2 (Utilities|Time|GetTimeSeconds))
  (bind _returnvalue_3 (Utilities|Time|GetTimeSeconds))
  (bind _returnvalue_4 (Utilities|Time|GetTimeSeconds))
  (bind _nohominggravityturn (Variables|Default|GetNoHomingGravityTurn))
  (bind _hominggravityturn (Variables|Default|GetHomingGravityTurn))
  (bind _hominggravityturn_2 (Variables|Default|GetHomingGravityTurn))
  (bind _homingnogravityturn (Variables|Default|GetHomingNoGravityTurn))
  (bind _nohomingnogravityturn (Variables|Default|GetNoHomingNoGravityTurn))
  (bind _homingnogravitynoturn (Variables|Default|GetHomingNoGravityNoTurn))
  (bind _homingnogravityturn_2 (Variables|Default|GetHomingNoGravityTurn))
  (bind _hominggravitynoturn (Variables|Default|GetHomingGravityNoTurn))
  (bind _outactors (Actor|GetAllActorsOfClass "/Game/My/BP/Play/Second/BP_PlaySecondGunBallProcess.BP_PlaySecondGunBallProcess_C"))
  (for _array_element _outactors
    (Variables|Default|SetBP_PlaysecondGunBallProcess _array_element))
  (if (Variables|/Game/My/BP/Play/Second/BP_PlaySecondGunBallProcess.BP_PlaySecondGunBallProcess_C|GetColor (Variables|Default|GetBP_PlaysecondGunBallProcess))
    ;[1 1 1] 色変更処理
    (bind _returnvalue_5 (Rendering|Material|CreateDynamicMaterialInstance (Variables|Default|GetSphere) 0 "/Game/My/Material/M_Rainbow.M_Rainbow" "None" :!class /Script/Engine.PrimitiveComponent))
    (Rendering|Material|SetVectorParameterValue _returnvalue_5 "Param" (Math|Color|MakeColor (Math|Random|RandomFloat) (Math|Random|RandomFloat) (Math|Random|RandomFloat)) :!class /Script/Engine.MaterialInstanceDynamic))
  (if (Variables|/Game/My/BP/Play/Second/BP_PlaySecondGunBallProcess.BP_PlaySecondGunBallProcess_C|GetMove (Variables|Default|GetBP_PlaysecondGunBallProcess))
    (if (Variables|/Game/My/BP/Play/Second/BP_PlaySecondGunBallProcess.BP_PlaySecondGunBallProcess_C|GetGravity (Variables|Default|GetBP_PlaysecondGunBallProcess))
      (if (Variables|/Game/My/BP/Play/Second/BP_PlaySecondGunBallProcess.BP_PlaySecondGunBallProcess_C|GetHoming (Variables|Default|GetBP_PlaysecondGunBallProcess))
        (if (Variables|/Game/My/BP/Play/Second/BP_PlaySecondGunBallProcess.BP_PlaySecondGunBallProcess_C|GetTurn (Variables|Default|GetBP_PlaysecondGunBallProcess))
          ;[1 1 1] 重力あってホーミングして回る場合
          (Components|Activation|SetActive (Variables|Default|GetNoHomingGravityNoTurn) false false)
          (Components|Activation|SetActive (Variables|Default|GetNoHomingNoGravityNoTurn) false false)
          (Components|Activation|SetActive (Variables|Default|GetHomingNoGravityNoTurn) false false)
          (Components|Activation|SetActive (Variables|Default|GetHomingGravityNoTurn) false false)
          (Components|Activation|SetActive (Variables|Default|GetNoHomingGravityTurn) false false)
          (Components|Activation|SetActive (Variables|Default|GetNoHomingNoGravityTurn) false false)
          (Components|Activation|SetActive (Variables|Default|GetHomingNoGravityTurn) false false)
          (Components|Activation|SetActive (Variables|Default|GetHomingGravityTurn) true false)
          ;[1 1 1] 回る処理
          (Variables|/Script/Engine.MovementComponent|SetVelocity _hominggravityturn (+ (Math|Vector|MakeVector (* (Math|Trig|Cos(Radians) _returnvalue) 1e+02) 1.0 (* (Math|Trig|Sin(Radians) _returnvalue) 1e+02)) (Variables|/Script/Engine.MovementComponent|GetVelocity _hominggravityturn)))
          ;[1 1 1] ホーミング処理
          (bind _outactors_2 (Actor|GetAllActorsOfClass "/Game/My/BP/Play/Second/BP_PlaySecondTarget.BP_PlaySecondTarget_C"))
          (for _array_element_2 _outactors_2
            (bind _returnvalue_6 (AddComponent|AddSceneComponent _array_element_2 false (Transformation|GetActorTransform _array_element_2)))
            (Variables|/Script/Engine.ProjectileMovementComponent|SetHomingTargetComponent (Variables|Default|GetHomingGravityTurn) _returnvalue_6)
            (if (>= (.x (Transformation|GetActorLocation _array_element_2)) (.x (Transformation|GetActorLocation)))
              (Variables|/Script/Engine.ProjectileMovementComponent|SetHomingAccelerationMagnitude _hominggravityturn_2 -5e+02)
              (else
                (Variables|/Script/Engine.ProjectileMovementComponent|SetHomingAccelerationMagnitude _hominggravityturn_2 5e+02))))
          (else
            ;[1 1 1] 重力あってホーミングして回らない場合
            (Components|Activation|SetActive (Variables|Default|GetNoHomingGravityNoTurn) false false)
            (Components|Activation|SetActive (Variables|Default|GetNoHomingNoGravityNoTurn) false false)
            (Components|Activation|SetActive (Variables|Default|GetHomingNoGravityNoTurn) false false)
            (Components|Activation|SetActive (Variables|Default|GetHomingGravityTurn) false false)
            (Components|Activation|SetActive (Variables|Default|GetNoHomingGravityTurn) false false)
            (Components|Activation|SetActive (Variables|Default|GetNoHomingNoGravityTurn) false false)
            (Components|Activation|SetActive (Variables|Default|GetHomingNoGravityTurn) false false)
            (Components|Activation|SetActive (Variables|Default|GetHomingGravityNoTurn) true false)
            ;[1 1 1] ホーミング処理
            (bind _outactors_3 (Actor|GetAllActorsOfClass "/Game/My/BP/Play/Second/BP_PlaySecondTarget.BP_PlaySecondTarget_C"))
            (for _array_element_3 _outactors_3
              (bind _returnvalue_7 (AddComponent|AddSceneComponent _array_element_3 false (Transformation|GetActorTransform _array_element_3)))
              (Variables|/Script/Engine.ProjectileMovementComponent|SetHomingTargetComponent (Variables|Default|GetHomingGravityNoTurn) _returnvalue_7)
              (if (>= (.x (Transformation|GetActorLocation _array_element_3)) (.x (Transformation|GetActorLocation)))
                (Variables|/Script/Engine.ProjectileMovementComponent|SetHomingAccelerationMagnitude _hominggravitynoturn -5e+02)
                (else
                  (Variables|/Script/Engine.ProjectileMovementComponent|SetHomingAccelerationMagnitude _hominggravitynoturn 5e+02))))))
        (elif (Variables|/Game/My/BP/Play/Second/BP_PlaySecondGunBallProcess.BP_PlaySecondGunBallProcess_C|GetTurn (Variables|Default|GetBP_PlaysecondGunBallProcess))
          ;[1 1 1] 重力あってホーミングしなくて回る場合
          (Components|Activation|SetActive (Variables|Default|GetNoHomingGravityNoTurn) false false)
          (Components|Activation|SetActive (Variables|Default|GetNoHomingNoGravityNoTurn) false false)
          (Components|Activation|SetActive (Variables|Default|GetHomingNoGravityNoTurn) false false)
          (Components|Activation|SetActive (Variables|Default|GetHomingGravityNoTurn) false false)
          (Components|Activation|SetActive (Variables|Default|GetNoHomingNoGravityTurn) false false)
          (Components|Activation|SetActive (Variables|Default|GetHomingNoGravityTurn) false false)
          (Components|Activation|SetActive (Variables|Default|GetHomingGravityTurn) false false)
          (Components|Activation|SetActive (Variables|Default|GetNoHomingGravityTurn) true false)
          ;[1 1 1] 回る処理
          (Variables|/Script/Engine.MovementComponent|SetVelocity _nohominggravityturn (+ (Math|Vector|MakeVector (* (Math|Trig|Cos(Radians) _returnvalue_4) 1e+02) 1.0 (* (Math|Trig|Sin(Radians) _returnvalue_4) 1e+02)) (Variables|/Script/Engine.MovementComponent|GetVelocity _nohominggravityturn)))
          (else
            ;[1 1 1] 重力あってホーミングしなくて回らない場合
            (Components|Activation|SetActive (Variables|Default|GetNoHomingNoGravityNoTurn) false false)
            (Components|Activation|SetActive (Variables|Default|GetHomingNoGravityNoTurn) false false)
            (Components|Activation|SetActive (Variables|Default|GetHomingGravityNoTurn) false false)
            (Components|Activation|SetActive (Variables|Default|GetNoHomingGravityTurn) false false)
            (Components|Activation|SetActive (Variables|Default|GetNoHomingNoGravityTurn) false false)
            (Components|Activation|SetActive (Variables|Default|GetHomingNoGravityTurn) false false)
            (Components|Activation|SetActive (Variables|Default|GetHomingGravityTurn) false false)
            (Components|Activation|SetActive (Variables|Default|GetNoHomingGravityNoTurn) true false))))
      (elif (Variables|/Game/My/BP/Play/Second/BP_PlaySecondGunBallProcess.BP_PlaySecondGunBallProcess_C|GetHoming (Variables|Default|GetBP_PlaysecondGunBallProcess))
        (if (Variables|/Game/My/BP/Play/Second/BP_PlaySecondGunBallProcess.BP_PlaySecondGunBallProcess_C|GetTurn (Variables|Default|GetBP_PlaysecondGunBallProcess))
          ;[1 1 1] 重力なくてホーミングして回る場合
          (Components|Activation|SetActive (Variables|Default|GetNoHomingGravityNoTurn) false false)
          (Components|Activation|SetActive (Variables|Default|GetNoHomingNoGravityNoTurn) false false)
          (Components|Activation|SetActive (Variables|Default|GetHomingNoGravityNoTurn) false false)
          (Components|Activation|SetActive (Variables|Default|GetHomingGravityNoTurn) false false)
          (Components|Activation|SetActive (Variables|Default|GetNoHomingGravityTurn) false false)
          (Components|Activation|SetActive (Variables|Default|GetNoHomingNoGravityTurn) false false)
          (Components|Activation|SetActive (Variables|Default|GetHomingGravityTurn) false false)
          (Components|Activation|SetActive (Variables|Default|GetHomingNoGravityTurn) true false)
          ;[1 1 1] 回る処理
          (Variables|/Script/Engine.MovementComponent|SetVelocity _homingnogravityturn (+ (Math|Vector|MakeVector (* (Math|Trig|Cos(Radians) _returnvalue_3) 1e+02) 1.0 (* (Math|Trig|Sin(Radians) _returnvalue_3) 1e+02)) (Variables|/Script/Engine.MovementComponent|GetVelocity _homingnogravityturn)))
          ;[1 1 1] ホーミング処理
          (bind _outactors_4 (Actor|GetAllActorsOfClass "/Game/My/BP/Play/Second/BP_PlaySecondTarget.BP_PlaySecondTarget_C"))
          (for _array_element_4 _outactors_4
            (bind _returnvalue_8 (AddComponent|AddSceneComponent _array_element_4 false (Transformation|GetActorTransform _array_element_4)))
            (Variables|/Script/Engine.ProjectileMovementComponent|SetHomingTargetComponent (Variables|Default|GetHomingNoGravityTurn) _returnvalue_8)
            (if (>= (.x (Transformation|GetActorLocation _array_element_4)) (.x (Transformation|GetActorLocation)))
              (Variables|/Script/Engine.ProjectileMovementComponent|SetHomingAccelerationMagnitude _homingnogravityturn_2 -5e+02)
              (else
                (Variables|/Script/Engine.ProjectileMovementComponent|SetHomingAccelerationMagnitude _homingnogravityturn_2 5e+02))))
          (else
            ;[1 1 1] 重力なくてホーミングして回らない場合
            (Components|Activation|SetActive (Variables|Default|GetNoHomingGravityNoTurn) false false)
            (Components|Activation|SetActive (Variables|Default|GetNoHomingNoGravityNoTurn) false false)
            (Components|Activation|SetActive (Variables|Default|GetHomingGravityNoTurn) false false)
            (Components|Activation|SetActive (Variables|Default|GetNoHomingGravityTurn) false false)
            (Components|Activation|SetActive (Variables|Default|GetNoHomingNoGravityTurn) false false)
            (Components|Activation|SetActive (Variables|Default|GetHomingNoGravityTurn) false false)
            (Components|Activation|SetActive (Variables|Default|GetHomingGravityTurn) false false)
            (Components|Activation|SetActive (Variables|Default|GetHomingNoGravityNoTurn) true false)
            ;[1 1 1] ホーミング処理
            (bind _outactors_5 (Actor|GetAllActorsOfClass "/Game/My/BP/Play/Second/BP_PlaySecondTarget.BP_PlaySecondTarget_C"))
            (for _array_element_5 _outactors_5
              (bind _returnvalue_9 (AddComponent|AddSceneComponent _array_element_5 false (Transformation|GetActorTransform _array_element_5)))
              (Variables|/Script/Engine.ProjectileMovementComponent|SetHomingTargetComponent (Variables|Default|GetHomingNoGravityNoTurn) _returnvalue_9)
              (if (>= (.x (Transformation|GetActorLocation _array_element_5)) (.x (Transformation|GetActorLocation)))
                (Variables|/Script/Engine.ProjectileMovementComponent|SetHomingAccelerationMagnitude _homingnogravitynoturn -5e+02)
                (else
                  (Variables|/Script/Engine.ProjectileMovementComponent|SetHomingAccelerationMagnitude _homingnogravitynoturn 5e+02))))))
        (elif (Variables|/Game/My/BP/Play/Second/BP_PlaySecondGunBallProcess.BP_PlaySecondGunBallProcess_C|GetTurn (Variables|Default|GetBP_PlaysecondGunBallProcess))
          ;[1 1 1] 重力なくてホーミングしなくて回る場合
          (Components|Activation|SetActive (Variables|Default|GetNoHomingGravityNoTurn) false false)
          (Components|Activation|SetActive (Variables|Default|GetNoHomingNoGravityNoTurn) false false)
          (Components|Activation|SetActive (Variables|Default|GetHomingNoGravityNoTurn) false false)
          (Components|Activation|SetActive (Variables|Default|GetHomingGravityNoTurn) false false)
          (Components|Activation|SetActive (Variables|Default|GetNoHomingGravityTurn) false false)
          (Components|Activation|SetActive (Variables|Default|GetHomingNoGravityTurn) false false)
          (Components|Activation|SetActive (Variables|Default|GetHomingGravityTurn) false false)
          (Components|Activation|SetActive (Variables|Default|GetNoHomingNoGravityTurn) true false)
          ;[1 1 1] 回る処理
          (Variables|/Script/Engine.MovementComponent|SetVelocity _nohomingnogravityturn (+ (Math|Vector|MakeVector (* (Math|Trig|Cos(Radians) _returnvalue_2) 1e+02) 1.0 (* (Math|Trig|Sin(Radians) _returnvalue_2) 1e+02)) (Variables|/Script/Engine.MovementComponent|GetVelocity _nohomingnogravityturn)))
          (else
            ;[1 1 1] 重力なくてホーミングしなくて回らない場合
            (Components|Activation|SetActive (Variables|Default|GetNoHomingGravityNoTurn) false false)
            (Components|Activation|SetActive (Variables|Default|GetHomingNoGravityNoTurn) false false)
            (Components|Activation|SetActive (Variables|Default|GetHomingGravityNoTurn) false false)
            (Components|Activation|SetActive (Variables|Default|GetNoHomingGravityTurn) false false)
            (Components|Activation|SetActive (Variables|Default|GetNoHomingNoGravityTurn) false false)
            (Components|Activation|SetActive (Variables|Default|GetHomingNoGravityTurn) false false)
            (Components|Activation|SetActive (Variables|Default|GetHomingGravityTurn) false false)
            (Components|Activation|SetActive (Variables|Default|GetNoHomingNoGravityNoTurn) true false)))))
    (else
      ;[1 1 1] 動かない場合
      (Components|Activation|SetActive (Variables|Default|GetNoHomingGravityNoTurn) false false)
      (Components|Activation|SetActive (Variables|Default|GetNoHomingNoGravityNoTurn) false false)
      (Components|Activation|SetActive (Variables|Default|GetHomingNoGravityNoTurn) false false)
      (Components|Activation|SetActive (Variables|Default|GetHomingGravityNoTurn) false false)
      (Components|Activation|SetActive (Variables|Default|GetNoHomingGravityTurn) false false)
      (Components|Activation|SetActive (Variables|Default|GetNoHomingNoGravityTurn) false false)
      (Components|Activation|SetActive (Variables|Default|GetHomingNoGravityTurn) false false)
      (Components|Activation|SetActive (Variables|Default|GetHomingGravityTurn) false false))))

(event Collision|EventActorBeginOverlap
  (params (OtherActor :type Actor%20Object%20Reference)))

(event EventTick
  (params (DeltaSeconds :type Float%20%28single-precision%29))
  (if (Utilities|IsValid (Variables|Default|GetDefaultSceneRoot))
    (Utilities|FlowControl|Delay 7.0)
    (Actor|DestroyActor)))

(event Collision|EventHit
  (params (MyComp :type Primitive%20Component%20Object%20Reference) (Other :type Actor%20Object%20Reference) (OtherComp :type Primitive%20Component%20Object%20Reference) (bSelfMoved :type Boolean) (HitLocation :type Vector :default "0, 0, 0") (HitNormal :type Vector :default "0, 0, 0") (NormalImpulse :type Vector :default "0, 0, 0") (Hit :type Hit%20Result%20Structure%20%28by%20ref%29)))

(fn ConstructionScript)