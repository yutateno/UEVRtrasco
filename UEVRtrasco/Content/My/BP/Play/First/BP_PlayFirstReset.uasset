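; BP_PlayFirstReset is a motion-controller-grabbable reset object for the first play level.
; On BeginPlay it finds the level's cube set checker and robot actors.
; When picked up while the robot's Do flag is off, it clears the checker's cube number and set arrays, destroys its spawned actors, and teleports the robot to a fixed start location.
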(event EventBeginPlay
  (bind _outactors (Actor|GetAllActorsOfClass "/Game/My/BP/Play/First/BP_PlayFirstCubeSetCheck.BP_PlayFirstCubeSetCheck_C"))
  (for _array_element _outactors
    (Variables|Default|SetBP_PlayFirstCubeSetCheck _array_element))
  (bind _outactors_2 (Actor|GetAllActorsOfClass "/Game/My/BP/Play/First/BP_PlayFirstRobot.BP_PlayFirstRobot_C"))
  (for _array_element_2 _outactors_2
    (Variables|Default|SetBP_PlayFirstRobot _array_element_2)))

(event Collision|EventActorBeginOverlap
  (params (OtherActor :type Actor%20Object%20Reference)))

(event EventTick
  (params (DeltaSeconds :type Float%20%28single-precision%29)))

(event EventPickup
  (params (AttachTo :type Scene%20Component%20Object%20Reference))
  (bind _bp_playfirstcubesetcheck (Variables|Default|GetBP_PlayFirstCubeSetCheck))
  (bind _spawnactorarray (Variables|/Game/My/BP/Play/First/BP_PlayFirstCubeSetCheck.BP_PlayFirstCubeSetCheck_C|GetSpawnActorArray _bp_playfirstcubesetcheck))
  (if (not (Variables|/Game/My/BP/Play/First/BP_PlayFirstDo.BP_PlayFirstDo_C|GetDo (Variables|/Game/My/BP/Play/First/BP_PlayFirstRobot.BP_PlayFirstRobot_C|GetBP_PlayFirstDo (Variables|Default|GetBP_PlayFirstRobot))))
    (Utilities|Array|Clear (Variables|/Game/My/BP/Play/First/BP_PlayFirstCubeSetCheck.BP_PlayFirstCubeSetCheck_C|GetNumberCube _bp_playfirstcubesetcheck))
    (Utilities|Array|Clear (Variables|/Game/My/BP/Play/First/BP_PlayFirstCubeSetCheck.BP_PlayFirstCubeSetCheck_C|GetIsSet _bp_playfirstcubesetcheck))
    (bind _arrayelement (Utilities|Array|ReverseforEachLoop _spawnactorarray)
      (:LoopBody
        (if (Utilities|IsValid _arrayelement)
          (Actor|DestroyActor _arrayelement)))
      (:Completed
        (Utilities|Array|Clear _spawnactorarray)
        (Transformation|SetActorTransform (Variables|Default|GetBP_PlayFirstRobot) (Math|Transform|MakeTransform "-6057.000000,-810.000000,460.000000" "0, 0, 0" "1,1,1"))))))

(event EventDrop)

(fn ConstructionScript)