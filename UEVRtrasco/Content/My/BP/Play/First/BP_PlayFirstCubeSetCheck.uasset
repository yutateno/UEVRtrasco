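; Actor that spawns the command cubes (FrontMove, RightTurn, LeftTurn) into a grid of four columns with eight rows each.
; Every Tick it scans IsSet, flags each unset slot as set, and reads that slot's NumberCube value to pick the cube class.
; The slot index divided by 8 selects the column's Y, and the remainder steps Z downward.
; Each spawned cube is half-scale and is stored in SpawnActorArray.
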(event EventBeginPlay)

(event Collision|EventActorBeginOverlap
  (params (OtherActor :type Actor%20Object%20Reference)))

(event EventTick
  (params (DeltaSeconds :type Float%20%28single-precision%29))
  ;[1 1 1] マップの配列分ループをさせ、配置しているかどうかのフラッグにて配置されていないと分かったら次に進ませる
  (for (_array_element _array_index) (Variables|Default|GetIsSet)
    (if (not _array_element)
      (bind _output_get (Variables|Default|SetArryaNum _array_index))
      (Utilities|Array|SetArrayElem (Variables|Default|GetIsSet) _output_get true)
      ;[1 1 1] マップのkeyの値からどのブロックを配置するか調べる
      (if (== (Utilities|Array|Get(acopy) (Variables|Default|GetNumberCube) (Variables|Default|GetArryaNum)) 1)
        ;[1 1 1] FrontMoveを配置する
        (if (== (/ (Variables|Default|GetArryaNum) 8) 0)
          ;;[1 1 1] 一列目の時
          (bind _returnvalue (Game|SpawnActorfromClass "/Game/My/BP/Play/First/BP_PlayFirst_Cube_FrontMove.BP_PlayFirst_Cube_FrontMove_C" (Math|Transform|MakeTransform (Math|Vector|MakeVector (Math|Conversions|ToFloat(Integer) (Variables|Default|GetCubeAreaX)) (Math|Conversions|ToFloat(Integer) (Variables|Default|GetCubeOneAreaY)) (Math|Conversions|ToFloat(Integer) (- (Variables|Default|GetCubeOneAreaZ) (* (Variables|Default|GetArryaNum) (Variables|Default|GetCubeMultiAreaZ))))) "0, 0, 0" "0.500000,0.500000,0.500000") "Undefined" 0 0))
          (Utilities|Array|Add (Variables|Default|GetSpawnActorArray) _returnvalue)
          (elif (== (/ (Variables|Default|GetArryaNum) 8) 1)
            ;;[1 1 1] 二列目の時
            (bind _returnvalue_2 (Game|SpawnActorfromClass "/Game/My/BP/Play/First/BP_PlayFirst_Cube_FrontMove.BP_PlayFirst_Cube_FrontMove_C" (Math|Transform|MakeTransform (Math|Vector|MakeVector (Math|Conversions|ToFloat(Integer) (Variables|Default|GetCubeAreaX)) (Math|Conversions|ToFloat(Integer) (Variables|Default|GetCubeTwoAreaY)) (Math|Conversions|ToFloat(Integer) (- (Variables|Default|GetCubeOneAreaZ) (* (- (Variables|Default|GetArryaNum) 8) (Variables|Default|GetCubeMultiAreaZ))))) "0, 0, 0" "0.500000,0.500000,0.500000") "Undefined" 0 0))
            (Utilities|Array|Add (Variables|Default|GetSpawnActorArray) _returnvalue_2)
            (elif (== (/ (Variables|Default|GetArryaNum) 8) 2)
              ;;[1 1 1] 三列目の時
              (bind _returnvalue_3 (Game|SpawnActorfromClass "/Game/My/BP/Play/First/BP_PlayFirst_Cube_FrontMove.BP_PlayFirst_Cube_FrontMove_C" (Math|Transform|MakeTransform (Math|Vector|MakeVector (Math|Conversions|ToFloat(Integer) (Variables|Default|GetCubeAreaX)) (Math|Conversions|ToFloat(Integer) (Variables|Default|GetCubeThreeAreaY)) (Math|Conversions|ToFloat(Integer) (- (Variables|Default|GetCubeOneAreaZ) (* (- (Variables|Default|GetArryaNum) 16) (Variables|Default|GetCubeMultiAreaZ))))) "0, 0, 0" "0.500000,0.500000,0.500000") "Undefined" 0 0))
              (Utilities|Array|Add (Variables|Default|GetSpawnActorArray) _returnvalue_3)
              (elif (== (/ (Variables|Default|GetArryaNum) 8) 3)
                ;;[1 1 1] 四列目の時
                (bind _returnvalue_4 (Game|SpawnActorfromClass "/Game/My/BP/Play/First/BP_PlayFirst_Cube_FrontMove.BP_PlayFirst_Cube_FrontMove_C" (Math|Transform|MakeTransform (Math|Vector|MakeVector (Math|Conversions|ToFloat(Integer) (Variables|Default|GetCubeAreaX)) (Math|Conversions|ToFloat(Integer) (Variables|Default|GetCubeFourAreaY)) (Math|Conversions|ToFloat(Integer) (- (Variables|Default|GetCubeOneAreaZ) (* (- (Variables|Default|GetArryaNum) 24) (Variables|Default|GetCubeMultiAreaZ))))) "0, 0, 0" "0.500000,0.500000,0.500000") "Undefined" 0 0))
                (Utilities|Array|Add (Variables|Default|GetSpawnActorArray) _returnvalue_4)))))
        (elif (== (Utilities|Array|Get(acopy) (Variables|Default|GetNumberCube) (Variables|Default|GetArryaNum)) 2)
          ;[1 1 1] RightTurnを配置する
          (if (== (/ (Variables|Default|GetArryaNum) 8) 0)
            ;;[1 1 1] 一列目の時
            (bind _returnvalue_5 (Game|SpawnActorfromClass "/Game/My/BP/Play/First/BP_PlayFirst_Cube_RightTurn.BP_PlayFirst_Cube_RightTurn_C" (Math|Transform|MakeTransform (Math|Vector|MakeVector (Math|Conversions|ToFloat(Integer) (Variables|Default|GetCubeAreaX)) (Math|Conversions|ToFloat(Integer) (Variables|Default|GetCubeOneAreaY)) (Math|Conversions|ToFloat(Integer) (- (Variables|Default|GetCubeOneAreaZ) (* (Variables|Default|GetArryaNum) (Variables|Default|GetCubeMultiAreaZ))))) "0, 0, 0" "0.500000,0.500000,0.500000") "Undefined" 0 0))
            (Utilities|Array|Add (Variables|Default|GetSpawnActorArray) _returnvalue_5)
            (elif (== (/ (Variables|Default|GetArryaNum) 8) 1)
              ;;[1 1 1] 二列目の時
              (bind _returnvalue_6 (Game|SpawnActorfromClass "/Game/My/BP/Play/First/BP_PlayFirst_Cube_RightTurn.BP_PlayFirst_Cube_RightTurn_C" (Math|Transform|MakeTransform (Math|Vector|MakeVector (Math|Conversions|ToFloat(Integer) (Variables|Default|GetCubeAreaX)) (Math|Conversions|ToFloat(Integer) (Variables|Default|GetCubeTwoAreaY)) (Math|Conversions|ToFloat(Integer) (- (Variables|Default|GetCubeOneAreaZ) (* (- (Variables|Default|GetArryaNum) 8) (Variables|Default|GetCubeMultiAreaZ))))) "0, 0, 0" "0.500000,0.500000,0.500000") "Undefined" 0 0))
              (Utilities|Array|Add (Variables|Default|GetSpawnActorArray) _returnvalue_6)
              (elif (== (/ (Variables|Default|GetArryaNum) 8) 2)
                ;;[1 1 1] 三列目の時
                (bind _returnvalue_7 (Game|SpawnActorfromClass "/Game/My/BP/Play/First/BP_PlayFirst_Cube_RightTurn.BP_PlayFirst_Cube_RightTurn_C" (Math|Transform|MakeTransform (Math|Vector|MakeVector (Math|Conversions|ToFloat(Integer) (Variables|Default|GetCubeAreaX)) (Math|Conversions|ToFloat(Integer) (Variables|Default|GetCubeThreeAreaY)) (Math|Conversions|ToFloat(Integer) (- (Variables|Default|GetCubeOneAreaZ) (* (- (Variables|Default|GetArryaNum) 16) (Variables|Default|GetCubeMultiAreaZ))))) "0, 0, 0" "0.500000,0.500000,0.500000") "Undefined" 0 0))
                (Utilities|Array|Add (Variables|Default|GetSpawnActorArray) _returnvalue_7)
                (elif (== (/ (Variables|Default|GetArryaNum) 8) 3)
                  ;;[1 1 1] 四列目の時
                  (bind _returnvalue_8 (Game|SpawnActorfromClass "/Game/My/BP/Play/First/BP_PlayFirst_Cube_RightTurn.BP_PlayFirst_Cube_RightTurn_C" (Math|Transform|MakeTransform (Math|Vector|MakeVector (Math|Conversions|ToFloat(Integer) (Variables|Default|GetCubeAreaX)) (Math|Conversions|ToFloat(Integer) (Variables|Default|GetCubeFourAreaY)) (Math|Conversions|ToFloat(Integer) (- (Variables|Default|GetCubeOneAreaZ) (* (- (Variables|Default|GetArryaNum) 24) (Variables|Default|GetCubeMultiAreaZ))))) "0, 0, 0" "0.500000,0.500000,0.500000") "Undefined" 0 0))
                  (Utilities|Array|Add (Variables|Default|GetSpawnActorArray) _returnvalue_8)))))
          (elif (== (Utilities|Array|Get(acopy) (Variables|Default|GetNumberCube) (Variables|Default|GetArryaNum)) 3)
            ;[1 1 1] RightTurnを配置する
            (if (== (/ (Variables|Default|GetArryaNum) 8) 0)
              ;;[1 1 1] 一列目の時
              (bind _returnvalue_9 (Game|SpawnActorfromClass "/Game/My/BP/Play/First/BP_PlayFirst_Cube_LeftTurn.BP_PlayFirst_Cube_LeftTurn_C" (Math|Transform|MakeTransform (Math|Vector|MakeVector (Math|Conversions|ToFloat(Integer) (Variables|Default|GetCubeAreaX)) (Math|Conversions|ToFloat(Integer) (Variables|Default|GetCubeOneAreaY)) (Math|Conversions|ToFloat(Integer) (- (Variables|Default|GetCubeOneAreaZ) (* (Variables|Default|GetArryaNum) (Variables|Default|GetCubeMultiAreaZ))))) "0, 0, 0" "0.500000,0.500000,0.500000") "Undefined" 0 0))
              (Utilities|Array|Add (Variables|Default|GetSpawnActorArray) _returnvalue_9)
              (elif (== (/ (Variables|Default|GetArryaNum) 8) 1)
                ;;[1 1 1] 二列目の時
                (bind _returnvalue_10 (Game|SpawnActorfromClass "/Game/My/BP/Play/First/BP_PlayFirst_Cube_LeftTurn.BP_PlayFirst_Cube_LeftTurn_C" (Math|Transform|MakeTransform (Math|Vector|MakeVector (Math|Conversions|ToFloat(Integer) (Variables|Default|GetCubeAreaX)) (Math|Conversions|ToFloat(Integer) (Variables|Default|GetCubeTwoAreaY)) (Math|Conversions|ToFloat(Integer) (- (Variables|Default|GetCubeOneAreaZ) (* (- (Variables|Default|GetArryaNum) 8) (Variables|Default|GetCubeMultiAreaZ))))) "0, 0, 0" "0.500000,0.500000,0.500000") "Undefined" 0 0))
                (Utilities|Array|Add (Variables|Default|GetSpawnActorArray) _returnvalue_10)
                (elif (== (/ (Variables|Default|GetArryaNum) 8) 2)
                  ;;[1 1 1] 三列目の時
                  (bind _returnvalue_11 (Game|SpawnActorfromClass "/Game/My/BP/Play/First/BP_PlayFirst_Cube_LeftTurn.BP_PlayFirst_Cube_LeftTurn_C" (Math|Transform|MakeTransform (Math|Vector|MakeVector (Math|Conversions|ToFloat(Integer) (Variables|Default|GetCubeAreaX)) (Math|Conversions|ToFloat(Integer) (Variables|Default|GetCubeThreeAreaY)) (Math|Conversions|ToFloat(Integer) (- (Variables|Default|GetCubeOneAreaZ) (* (- (Variables|Default|GetArryaNum) 16) (Variables|Default|GetCubeMultiAreaZ))))) "0, 0, 0" "0.500000,0.500000,0.500000") "Undefined" 0 0))
                  (Utilities|Array|Add (Variables|Default|GetSpawnActorArray) _returnvalue_11)
                  (elif (== (/ (Variables|Default|GetArryaNum) 8) 3)
                    ;;[1 1 1] 四列目の時
                    (bind _returnvalue_12 (Game|SpawnActorfromClass "/Game/My/BP/Play/First/BP_PlayFirst_Cube_LeftTurn.BP_PlayFirst_Cube_LeftTurn_C" (Math|Transform|MakeTransform (Math|Vector|MakeVector (Math|Conversions|ToFloat(Integer) (Variables|Default|GetCubeAreaX)) (Math|Conversions|ToFloat(Integer) (Variables|Default|GetCubeFourAreaY)) (Math|Conversions|ToFloat(Integer) (- (Variables|Default|GetCubeOneAreaZ) (* (- (Variables|Default|GetArryaNum) 24) (Variables|Default|GetCubeMultiAreaZ))))) "0, 0, 0" "0.500000,0.500000,0.500000") "Undefined" 0 0))
                    (Utilities|Array|Add (Variables|Default|GetSpawnActorArray) _returnvalue_12)))))))))))

(fn ConstructionScript)