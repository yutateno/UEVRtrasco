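; Robot actor for the first play stage that executes a queued command sequence on a grid when BP_PlayFirstDo's Do flag turns on.
; Tick uses a DoOnce to step through BP_PlayFirstCubeSetCheck's NumberCube array with ForLoopAddDelay, a macro that advances only on Next, allowing one-second delays.
; Each step moves the BP_PlayFirst_Cube_NowDo indicator, then moves forward by roll-based heading within bounds or rotates 90 degrees.
; Completion clears Do.
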(event EventBeginPlay
  (bind _outactors (Actor|GetAllActorsOfClass "/Game/My/BP/Play/First/BP_PlayFirstCubeSetCheck.BP_PlayFirstCubeSetCheck_C"))
  (for _array_element _outactors
    (Variables|Default|SetBP_PlayFirstCubeSetCheck _array_element))
  (bind _outactors_2 (Actor|GetAllActorsOfClass "/Game/My/BP/Play/First/BP_PlayFirstDo.BP_PlayFirstDo_C"))
  (for _array_element_2 _outactors_2
    (Variables|Default|SetBP_PlayFirstDo _array_element_2))
  (bind _outactors_3 (Actor|GetAllActorsOfClass "/Game/My/BP/Play/First/BP_PlayFirst_Cube_NowDo.BP_PlayFirst_Cube_NowDo_C"))
  (for _array_element_3 _outactors_3
    (Variables|Default|SetBP_PlayFirst_Cube_NowDo _array_element_3)))

(event Collision|EventActorBeginOverlap
  (params (OtherActor :type Actor%20Object%20Reference)))

(event EventTick
  (params (DeltaSeconds :type Float%20%28single-precision%29))
  (bind _bp_playfirst_cube_nowdo (Variables|Default|GetBP_PlayFirst_Cube_NowDo))
  (bind _bp_playfirst_cube_nowdo_2 (Variables|Default|GetBP_PlayFirst_Cube_NowDo))
  (bind _defaultsceneroot (Variables|Default|GetDefaultSceneRoot))
  (bind _defaultsceneroot_2 (Variables|Default|GetDefaultSceneRoot))
  (bind _defaultsceneroot_3 (Variables|Default|GetDefaultSceneRoot))
  (bind _defaultsceneroot_4 (Variables|Default|GetDefaultSceneRoot))
  (bind _defaultsceneroot_5 (Variables|Default|GetDefaultSceneRoot))
  (bind _defaultsceneroot_6 (Variables|Default|GetDefaultSceneRoot))
  (bind _bp_playfirst_cube_nowdo_3 (Variables|Default|GetBP_PlayFirst_Cube_NowDo))
  (bind _bp_playfirst_cube_nowdo_4 (Variables|Default|GetBP_PlayFirst_Cube_NowDo))
  (bind _returnvalue (Transformation|GetWorldRotation _defaultsceneroot_2))
  (bind _returnvalue_2 (Transformation|GetWorldRotation _defaultsceneroot))
  (bind _returnvalue_3 (Transformation|GetWorldLocation _defaultsceneroot_4))
  (bind _returnvalue_4 (Transformation|GetWorldLocation _defaultsceneroot_6))
  (bind _returnvalue_5 (Transformation|GetWorldLocation _defaultsceneroot_3))
  (bind _returnvalue_6 (Transformation|GetWorldLocation _defaultsceneroot_5))
  (bind _defaultsceneroot_7 (Variables|/Game/My/BP/Play/First/BP_PlayFirst_Cube_NowDo.BP_PlayFirst_Cube_NowDo_C|GetDefaultSceneRoot _bp_playfirst_cube_nowdo_4))
  (bind _defaultsceneroot_8 (Variables|/Game/My/BP/Play/First/BP_PlayFirst_Cube_NowDo.BP_PlayFirst_Cube_NowDo_C|GetDefaultSceneRoot _bp_playfirst_cube_nowdo_2))
  (bind _defaultsceneroot_9 (Variables|/Game/My/BP/Play/First/BP_PlayFirst_Cube_NowDo.BP_PlayFirst_Cube_NowDo_C|GetDefaultSceneRoot _bp_playfirst_cube_nowdo))
  (bind _defaultsceneroot_10 (Variables|/Game/My/BP/Play/First/BP_PlayFirst_Cube_NowDo.BP_PlayFirst_Cube_NowDo_C|GetDefaultSceneRoot _bp_playfirst_cube_nowdo_3))
  (if (Variables|/Game/My/BP/Play/First/BP_PlayFirstDo.BP_PlayFirstDo_C|GetDo (Variables|Default|GetBP_PlayFirstDo))
    (Utilities|FlowControl|DoOnce false :!label _label
      (:Completed
        (Variables|Default|SetArray%20Index -1)
        (bind _arrayelement (Utilities|ForLoopAddDelay (Variables|/Game/My/BP/Play/First/BP_PlayFirstCubeSetCheck.BP_PlayFirstCubeSetCheck_C|GetNumberCube (Variables|Default|GetBP_PlayFirstCubeSetCheck)) :!label _label_2)
          (:LoopBody
            (Math|Integer|IncrementInt (Variables|Default|GetArray%20Index)
              (:%20%20
                ;[1 1 1] 左の黄色いパネルの動き
                (if (== (/ (Variables|Default|GetArray%20Index) 8) 0)
                  (Transformation|SetWorldLocation _defaultsceneroot_10 (Math|Vector|MakeVector (.x (Transformation|GetWorldLocation _defaultsceneroot_10)) 107.0 (- 691.0 (* (Math|Conversions|ToFloat(Integer) (Variables|Default|GetArray%20Index)) 54.0))) false false)
                  (elif (== (/ (Variables|Default|GetArray%20Index) 8) 1)
                    (Transformation|SetWorldLocation _defaultsceneroot_7 (Math|Vector|MakeVector (.x (Transformation|GetWorldLocation _defaultsceneroot_7)) 19.0 (- 691.0 (* (Math|Conversions|ToFloat(Integer) (- (Variables|Default|GetArray%20Index) 8)) 54.0))) false false)
                    (elif (== (/ (Variables|Default|GetArray%20Index) 8) 2)
                      (Transformation|SetWorldLocation _defaultsceneroot_8 (Math|Vector|MakeVector (.x (Transformation|GetWorldLocation _defaultsceneroot_8)) -7e+01 (- 691.0 (* (Math|Conversions|ToFloat(Integer) (- (Variables|Default|GetArray%20Index) 16)) 54.0))) false false)
                      (elif (== (/ (Variables|Default|GetArray%20Index) 8) 3)
                        (Transformation|SetWorldLocation _defaultsceneroot_9 (Math|Vector|MakeVector (.x (Transformation|GetWorldLocation _defaultsceneroot_9)) -163.0 (- 691.0 (* (Math|Conversions|ToFloat(Integer) (- (Variables|Default|GetArray%20Index) 24)) 54.0))) false false)))))
                (Utilities|FlowControl|Delay 1.0)
                ;[1 1 1] 前方
                (if (== _arrayelement 1)
                  ;[1 1 1] 左方向に進む
                  (if (Math|Float|NearlyEqual(Float) (.roll (Transformation|GetWorldRotation (Variables|Default|GetDefaultSceneRoot))) 0.0 1.0)
                    (if (Math|Float|NearlyEqual(Float) (.y _returnvalue_4) -329.0 1.0)
                      (goto _label_2 Next)
                      (else
                        (Transformation|SetWorldLocation _defaultsceneroot_6 (Math|Vector|MakeVector (.x _returnvalue_4) (+ (.y _returnvalue_4) 96.0) (.z _returnvalue_4)) false false)
                        (goto _label_2 Next)))
                    (else
                      ;[1 1 1] 下方向に進む
                      (if (Math|Float|NearlyEqual(Float) (.roll (Transformation|GetWorldRotation (Variables|Default|GetDefaultSceneRoot))) 9e+01 1.0)
                        (if (Math|Float|NearlyEqual(Float) (.z _returnvalue_5) 3.7e+02 1.0)
                          (goto _label_2 Next)
                          (else
                            (Transformation|SetWorldLocation _defaultsceneroot_3 (Math|Vector|MakeVector (.x _returnvalue_5) (.y _returnvalue_5) (- (.z _returnvalue_5) 9e+01)) false false)
                            (goto _label_2 Next)))
                        (else
                          ;[1 1 1] 上方向に進む
                          (if (Math|Float|NearlyEqual(Float) (.roll (Transformation|GetWorldRotation (Variables|Default|GetDefaultSceneRoot))) -9e+01 1.0)
                            (if (Math|Float|NearlyEqual(Float) (.z _returnvalue_3) 6.4e+02 1.0)
                              (goto _label_2 Next)
                              (else
                                (Transformation|SetWorldLocation _defaultsceneroot_4 (Math|Vector|MakeVector (.x _returnvalue_3) (.y _returnvalue_3) (+ (.z _returnvalue_3) 9e+01)) false false)
                                (goto _label_2 Next)))
                            (else
                              ;[1 1 1] 右方向に進む
                              (if (Math|Float|NearlyEqual(Float) (.y _returnvalue_6) -8.1e+02 1.0)
                                (goto _label_2 Next)
                                (else
                                  (Transformation|SetWorldLocation _defaultsceneroot_5 (Math|Vector|MakeVector (.x _returnvalue_6) (- (.y _returnvalue_6) 96.0) (.z _returnvalue_6)) false false)
                                  (goto _label_2 Next)))))))))
                  (else
                    ;[1 1 1] 右回転
                    (if (== _arrayelement 2)
                      (Transformation|SetWorldRotation _defaultsceneroot_2 (Math|Rotator|MakeRotator (- (.roll _returnvalue) 9e+01) (.pitch _returnvalue) (.yaw _returnvalue)) false false)
                      (goto _label_2 Next)
                      (else
                        ;[1 1 1] 左回転
                        (if (== _arrayelement 3)
                          (Transformation|SetWorldRotation _defaultsceneroot (Math|Rotator|MakeRotator (+ (.roll _returnvalue_2) 9e+01) (.pitch _returnvalue_2) (.yaw _returnvalue_2)) false false)
                          (goto _label_2 Next)
                          (else
                            (goto _label_2 Next))))))))))
          (:Completed
            ;[1 1 1] ループ終了
            (Variables|/Game/My/BP/Play/First/BP_PlayFirstDo.BP_PlayFirstDo_C|SetDo (Variables|Default|GetBP_PlayFirstDo) false)))))
    (else
      (goto _label Reset))))

(fn ConstructionScript)