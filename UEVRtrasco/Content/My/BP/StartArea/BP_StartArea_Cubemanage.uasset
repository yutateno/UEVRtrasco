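; BP_StartArea_Cubemanage maintains a row of BP_PickupCube actors in the start area, replacing cubes that drop too low.
; BeginPlay spawns seven cubes spaced along Y from AreaY and stores them in an array.
; Tick flags any cube below a height threshold, and a DoOnce, reset while none is flagged, destroys it after a short delay.
; Replacements spawn at a cycling slot counter's position, not the removed cube's.
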(event EventBeginPlay
  (Utilities|Array|Clear (Variables|Default|GetBP_PicuUpCube))
  (for _index (range 0 6)
    (bind _returnvalue (Game|SpawnActorfromClass "/Game/VirtualRealityBP/Blueprints/BP_PickupCube.BP_PickupCube_C" (Math|Transform|MakeTransform (Math|Vector|MakeVector 547.821777 (+ (Variables|Default|GetAreaY) (* _index 4e+01)) 368.113007) "0, 0, 0" "1.000000,1.000000,1.000000") "Undefined" 0 0))
    (Utilities|Array|Add (Variables|Default|GetBP_PicuUpCube) _returnvalue)))

(event Collision|EventActorBeginOverlap
  (params (OtherActor :type Actor%20Object%20Reference)))

(event EventTick
  (params (DeltaSeconds :type Float%20%28single-precision%29))
  (for (_array_element _array_index) (Variables|Default|GetBP_PicuUpCube)
    (if (<= (.z (.location (Transformation|GetActorTransform _array_element))) 220.113007)
      (Variables|Default|SetNextDestroy _array_index)))
  (if (== (Variables|Default|GetNextDestroy) -1)
    (goto _label Reset)
    (else
      (Utilities|FlowControl|DoOnce false :!label _label
        (:Completed
          (Utilities|FlowControl|Delay 1.0)
          (for (_array_element_2 _array_index_2) (Variables|Default|GetBP_PicuUpCube)
            (if (== _array_index_2 (Variables|Default|GetNextDestroy))
              (Actor|DestroyActor _array_element_2)))
          (Utilities|Array|RemoveIndex (Variables|Default|GetBP_PicuUpCube) (Variables|Default|GetNextDestroy))
          (bind _result (Math|Integer|IncrementInt (Variables|Default|GetSpawnNum))
            (:%20%20
              (if (> _result 6)
                (Variables|Default|SetSpawnNum 0)
                (bind _returnvalue (Game|SpawnActorfromClass "/Game/VirtualRealityBP/Blueprints/BP_PickupCube.BP_PickupCube_C" (Math|Transform|MakeTransform (Math|Vector|MakeVector 547.821777 (Variables|Default|GetAreaY) 368.113007) "0, 0, 0" "1.000000,1.000000,1.000000") "Undefined" 0 0))
                (Utilities|Array|Add (Variables|Default|GetBP_PicuUpCube) _returnvalue)
                (else
                  (bind _returnvalue_2 (Game|SpawnActorfromClass "/Game/VirtualRealityBP/Blueprints/BP_PickupCube.BP_PickupCube_C" (Math|Transform|MakeTransform (Math|Vector|MakeVector 547.821777 (+ (Variables|Default|GetAreaY) (* (Variables|Default|GetSpawnNum) 4e+01)) 368.113007) "0, 0, 0" "1.000000,1.000000,1.000000") "Undefined" 0 0))
                  (Utilities|Array|Add (Variables|Default|GetBP_PicuUpCube) _returnvalue_2)))
              (Variables|Default|SetNextDestroy -1))))))))

(fn ConstructionScript)