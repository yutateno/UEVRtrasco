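; VR quiz trigger cube that, when picked up by the motion controller, shows a subtraction result as spawned cubes.
; Pickup destroys tracked cubes, then spawns numbered PickUpCubes for the Add actor's AddNum minus the Sub actor's SubNum.
; Cubes fill rows along Y, wrapping with a step down in X and Z.
; BeginPlay caches the Add and Sub actors and spawns a hardcoded test batch.
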(event EventBeginPlay
  (bind _outactors (Actor|GetAllActorsOfClass "/Game/My/BP/SecondObject/Quiz/FirstQuizPlay/BP_Cube_SecondFirstQuizAdd.BP_Cube_SecondFirstQuizAdd_C"))
  (for _array_element _outactors
    (Variables|Default|SetBP_Cube_SecondFirstQuizAdd _array_element)
    (bind _outactors_2 (Actor|GetAllActorsOfClass "/Game/My/BP/SecondObject/Quiz/FirstQuizPlay/BP_Cube_SecondFirstQuizSub.BP_Cube_SecondFirstQuizSub_C"))
    (for _array_element_2 _outactors_2
      (Variables|Default|SetBP_Cube_SecondFirstQuizSub _array_element_2)
      ;[1 1 1] Test
      (Variables|Default|SetTouchNum 20)
      (bind _result (Math|Integer|DecrementInt (Variables|Default|GetTouchNum))
        (:%20%20
          (if (>= _result 0)
            (for _index (range 0 _result)
              (bind _output_get (Variables|Default|SetAreaY (+ (Variables|Default|GetAreaY) 31.0)))
              (if (> _output_get 2279.0)
                (bind _output_get_2 (Variables|Default|SetAreaY 1.68e+03))
                (bind _output_get_3 (Variables|Default|SetAreaX (- (Variables|Default|GetAreaX) 21.0)))
                (bind _output_get_4 (Variables|Default|SetAreaZ (- (Variables|Default|GetAreaZ) 25.0)))
                (bind _returnvalue (Game|SpawnActorfromClass "/Game/My/BP/SecondObject/Quiz/FirstQuizPlay/BP_Cube_SecondFirstQuizPickUpCube.BP_Cube_SecondFirstQuizPickUpCube_C" (Math|Transform|MakeTransform (Math|Vector|MakeVector _output_get_3 _output_get_2 _output_get_4) "0, 0, 0" "1,1,1") "Undefined" 0 _index 0))
                (Utilities|Array|Add (Variables|Default|GetBP_Cube_SecondFirstQuizPickUpCubeArray) _returnvalue)
                (else
                  (bind _returnvalue_2 (Game|SpawnActorfromClass "/Game/My/BP/SecondObject/Quiz/FirstQuizPlay/BP_Cube_SecondFirstQuizPickUpCube.BP_Cube_SecondFirstQuizPickUpCube_C" (Math|Transform|MakeTransform (Math|Vector|MakeVector (Variables|Default|GetAreaX) _output_get (Variables|Default|GetAreaZ)) "0, 0, 0" "1,1,1") "Undefined" 0 _index 0))
                  (Utilities|Array|Add (Variables|Default|GetBP_Cube_SecondFirstQuizPickUpCubeArray) _returnvalue_2))))))))))

(event Collision|EventActorBeginOverlap
  (params (OtherActor :type Actor%20Object%20Reference)))

(event EventTick
  (params (DeltaSeconds :type Float%20%28single-precision%29)))

(event EventPickup
  (params (AttachTo :type Scene%20Component%20Object%20Reference))
  (bind _bp_cube_secondfirstquizpickupcubearray (Variables|Default|GetBP_Cube_SecondFirstQuizPickUpCubeArray))
  (Variables|Default|SetAreaY 1649.0)
  (Variables|Default|SetAreaX 7.03e+03)
  (Variables|Default|SetAreaZ 5e+02)
  (Variables|Default|SetTouchNum 0)
  (for (_array_element _array_index) _bp_cube_secondfirstquizpickupcubearray
    (if (Utilities|IsValid _array_element)
      (Actor|DestroyActor _array_element)
      (Utilities|Array|RemoveIndex _bp_cube_secondfirstquizpickupcubearray _array_index)))
  (bind _output_get (Variables|Default|SetTouchNum (Variables|/Game/My/BP/SecondObject/Quiz/FirstQuizPlay/BP_Cube_SecondFirstQuizAdd.BP_Cube_SecondFirstQuizAdd_C|GetAddNum (Variables|Default|GetBP_Cube_SecondFirstQuizAdd))))
  (Variables|Default|SetTouchNum (- _output_get (Variables|/Game/My/BP/SecondObject/Quiz/FirstQuizPlay/BP_Cube_SecondFirstQuizSub.BP_Cube_SecondFirstQuizSub_C|GetSubNum (Variables|Default|GetBP_Cube_SecondFirstQuizSub))))
  (bind _result (Math|Integer|DecrementInt (Variables|Default|GetTouchNum))
    (:%20%20
      (if (>= _result 0)
        (for _index (range 0 _result)
          (bind _output_get_2 (Variables|Default|SetAreaY (+ (Variables|Default|GetAreaY) 31.0)))
          (if (> _output_get_2 2279.0)
            (bind _output_get_3 (Variables|Default|SetAreaY 1.68e+03))
            (bind _output_get_4 (Variables|Default|SetAreaX (- (Variables|Default|GetAreaX) 21.0)))
            (bind _output_get_5 (Variables|Default|SetAreaZ (- (Variables|Default|GetAreaZ) 25.0)))
            (bind _returnvalue (Game|SpawnActorfromClass "/Game/My/BP/SecondObject/Quiz/FirstQuizPlay/BP_Cube_SecondFirstQuizPickUpCube.BP_Cube_SecondFirstQuizPickUpCube_C" (Math|Transform|MakeTransform (Math|Vector|MakeVector _output_get_4 _output_get_3 _output_get_5) "0, 0, 0" "1,1,1") "Undefined" 0 _index 0))
            (Utilities|Array|Add (Variables|Default|GetBP_Cube_SecondFirstQuizPickUpCubeArray) _returnvalue)
            (else
              (bind _returnvalue_2 (Game|SpawnActorfromClass "/Game/My/BP/SecondObject/Quiz/FirstQuizPlay/BP_Cube_SecondFirstQuizPickUpCube.BP_Cube_SecondFirstQuizPickUpCube_C" (Math|Transform|MakeTransform (Math|Vector|MakeVector (Variables|Default|GetAreaX) _output_get_2 (Variables|Default|GetAreaZ)) "0, 0, 0" "1,1,1") "Undefined" 0 _index 0))
              (Utilities|Array|Add (Variables|Default|GetBP_Cube_SecondFirstQuizPickUpCubeArray) _returnvalue_2))))))))

(event EventDrop)

(fn ConstructionScript)