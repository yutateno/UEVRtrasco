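; A numbered pickup cube actor for VR motion controllers, apparently part of the first quiz.
; On BeginPlay it creates one number widget from its Number value, assigns it to six widget components and disables physics.
; Pickup, called by BP_MotionController, attaches the cube to the supplied component with physics off.
; Drop and any mesh hit both re-enable physics and detach it, so a collision also releases a held cube.
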(event OnComponentHit(StaticMeshComponent)
  (params (HitComponent :type Primitive%20Component%20Object%20Reference) (OtherActor :type Actor%20Object%20Reference) (OtherComp :type Primitive%20Component%20Object%20Reference) (NormalImpulse :type Vector :default "0, 0, 0") (Hit :type Hit%20Result%20Structure%20%28by%20ref%29))
  (Physics|SetSimulatePhysics (Variables|Debug|GetStaticMeshComponent) true)
  (Transformation|DetachFromActor "KeepWorld" "KeepWorld" "KeepWorld"))

(event EventBeginPlay
  (Variables|Default|SetFlag false)
  (bind _returnvalue (UserInterface|CreateWidget "/Game/My/Widget/SecondObject/Quiz/First/Widget_Second_FirstCubeNumber.Widget_Second_FirstCubeNumber_C" 0 (Variables|Default|GetNumber)))
  (UserInterface|SetWidget (Variables|Default|GetWidget) _returnvalue)
  (UserInterface|SetWidget (Variables|Default|GetWidget1) _returnvalue)
  (UserInterface|SetWidget (Variables|Default|GetWidget2) _returnvalue)
  (UserInterface|SetWidget (Variables|Default|GetWidget3) _returnvalue)
  (UserInterface|SetWidget (Variables|Default|GetWidget4) _returnvalue)
  (UserInterface|SetWidget (Variables|Default|GetWidget5) _returnvalue)
  (Physics|SetSimulatePhysics (Variables|Debug|GetStaticMeshComponent) false))

(event Collision|EventActorBeginOverlap
  (params (OtherActor :type Actor%20Object%20Reference)))

(event EventTick
  (params (DeltaSeconds :type Float%20%28single-precision%29)))

(event EventPickup
  (params (AttachTo :type Scene%20Component%20Object%20Reference))
  (Physics|SetSimulatePhysics (Variables|Debug|GetStaticMeshComponent) false)
  (Transformation|AttachComponentToComponent (VehicleSound|GetRootComponent) AttachTo "None" "KeepWorld" "KeepWorld" "KeepWorld" false))

(event EventDrop
  (Physics|SetSimulatePhysics (Variables|Debug|GetStaticMeshComponent) true)
  (Transformation|DetachFromActor "KeepWorld" "KeepWorld" "KeepWorld"))

(fn ConstructionScript)