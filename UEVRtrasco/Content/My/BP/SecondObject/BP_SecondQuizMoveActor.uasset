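; BP_SecondQuizMoveActor is an actor that shuttles back and forth along the world X axis between two hard-coded bounds.
; Each Tick it sets the Turn flag at either limit, then offsets itself by a fixed step in that direction, so speed depends on frame rate.
; A hit on its Cube component also flips Turn and prints a debug string.
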(event OnComponentHit(Cube)
  (params (HitComponent :type Primitive%20Component%20Object%20Reference) (OtherActor :type Actor%20Object%20Reference) (OtherComp :type Primitive%20Component%20Object%20Reference) (NormalImpulse :type Vector :default "0, 0, 0") (Hit :type Hit%20Result%20Structure%20%28by%20ref%29))
  (Development|PrintString "Hello")
  (Variables|Default|SetTurn (not (Variables|Default|GetTurn))))

(event EventBeginPlay)

(event Collision|EventActorBeginOverlap
  (params (OtherActor :type Actor%20Object%20Reference)))

(event EventTick
  (params (DeltaSeconds :type Float%20%28single-precision%29))
  (bind _returnvalue (Transformation|GetActorLocation))
  (if (<= (.x _returnvalue) 7335.0)
    (Variables|Default|SetTurn true))
  (if (>= (.x _returnvalue) 10101.0)
    (Variables|Default|SetTurn false))
  (if (Variables|Default|GetTurn)
    (Transformation|AddActorWorldOffset (Math|Vector|MakeVector 1e+01 0.0 0.0))
    (else
      (Transformation|AddActorWorldOffset (Math|Vector|MakeVector -1e+01 0.0 0.0)))))

(fn ConstructionScript)