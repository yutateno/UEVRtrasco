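; Looping display actor that randomly presents an INT sphere or FLOAT cube, each with a widget, and sends it left or right.
; Tick starts each cycle behind a Do flag, with chained timeline Finished events sequencing reveal, slide and swap.
; The slide ends by spawning BP_First_INT for the sphere or BP_First_Float for the cube at that side's hardcoded position.
; A final timeline resets the component, destroys the spawned actor and clears Do to repeat.
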(event EventBeginPlay)

(event Collision|EventActorBeginOverlap
  (params (OtherActor :type Actor%20Object%20Reference)))

(event EventTick
  (params (DeltaSeconds :type Float%20%28single-precision%29))
  (bind _sphere (Variables|Default|GetSphere))
  (bind _cube (Variables|Default|GetCube))
  (if (not (Variables|Default|GetDo))
    (Variables|Default|SetDo true)
    (Variables|Default|SetIsSphereVisible false)
    (Development|SetHiddeninGame (Variables|Default|GetSphereWidget) true false)
    (Development|SetHiddeninGame (Variables|Default|GetSphere) true false)
    (Development|SetHiddeninGame (Variables|Default|GetCubeWidget) true false)
    (Development|SetHiddeninGame (Variables|Default|GetCube) true false)
    (Timeline|生成まで PlayFromStart
      (:Finished
        (if (Math|Random|RandomBool)
          (Development|SetHiddeninGame (Variables|Default|GetSphere) false false)
          (Development|SetHiddeninGame (Variables|Default|GetSphereWidget) false false)
          (Variables|Default|SetIsSphereVisible true)
          (Timeline|移動まで PlayFromStart
            (:Finished
              (if (Variables|Default|GetIsSphereVisible)
                (if (Math|Random|RandomBool)
                  (Components|MoveComponentTo _sphere "272.000000,0.000000,0.000000" "0, 0, 0" false false 1.0 false)
                  (Timeline|Int%20to%20Int PlayFromStart
                    (:Finished
                      (bind _returnvalue (Game|SpawnActorfromClass "/Game/My/BP/FirstObject/BP_First_INT.BP_First_INT_C" (Math|Transform|MakeTransform "2582.000000,1461.000000,599.000000" "0, 0, 0" "0.250000,0.250000,0.250000") "Undefined" 0 0))
                      (Variables|Default|SetBP_First_INT1 _returnvalue)))
                  (else
                    (Components|MoveComponentTo _sphere "-250.000000,0.000000,0.000000" "0, 0, 0" false false 1.0 false)
                    (Timeline|Int%20to%20Float PlayFromStart
                      (:Finished
                        (bind _returnvalue_2 (Game|SpawnActorfromClass "/Game/My/BP/FirstObject/BP_First_INT.BP_First_INT_C" (Math|Transform|MakeTransform "2060.000000,1461.000000,599.000000" "0, 0, 0" "0.250000,0.250000,0.250000") "Undefined" 0 0))
                        (Variables|Default|SetBP_First_INT2 _returnvalue_2)))))
                (Development|SetHiddeninGame (Variables|Default|GetSphere) true false)
                (Development|SetHiddeninGame (Variables|Default|GetSphereWidget) true false)
                (Timeline|Intを消すまで PlayFromStart
                  (:Finished
                    (Transformation|SetWorldLocation (Variables|Default|GetSphere) "2310.000000,1461.000000,590.000000" false false)
                    (if (Utilities|IsValid (Variables|Default|GetBP_First_INT1))
                      (Actor|DestroyActor (Variables|Default|GetBP_First_INT1))
                      (else
                        (Actor|DestroyActor (Variables|Default|GetBP_First_INT2))))))
                (else
                  (if (Math|Random|RandomBool)
                    (Components|MoveComponentTo _cube "272.000000,0.000000,0.000000" "0, 0, 0" false false 1.0 false)
                    (Timeline|Float%20to%20Int PlayFromStart
                      (:Finished
                        (bind _returnvalue_3 (Game|SpawnActorfromClass "/Game/My/BP/FirstObject/BP_First_Float.BP_First_Float_C" (Math|Transform|MakeTransform "2582.0,1461.000000,590.000000" "0, 0, 0" "1.100000,0.250000,0.250000") "Undefined" 0 0))
                        (Variables|Default|SetBP_First_FLOAT1 _returnvalue_3)))
                    (else
                      (Components|MoveComponentTo _cube "-250.000000,0.000000,0.000000" "0, 0, 0" false false 1.0 false)
                      (Timeline|Float%20to%20Float PlayFromStart
                        (:Finished
                          (bind _returnvalue_4 (Game|SpawnActorfromClass "/Game/My/BP/FirstObject/BP_First_Float.BP_First_Float_C" (Math|Transform|MakeTransform "2060.000000,1461.000000,590.000000" "0, 0, 0" "1.100000,0.250000,0.250000") "Undefined" 0 0))
                          (Variables|Default|SetBP_First_FLOAT2 _returnvalue_4)))))
                  (Development|SetHiddeninGame (Variables|Default|GetCube) true false)
                  (Development|SetHiddeninGame (Variables|Default|GetCubeWidget) true false)
                  (Timeline|Floatを消すまで PlayFromStart
                    (:Finished
                      (Transformation|SetWorldLocation (Variables|Default|GetCube) "2310.000000,1461.000000,590.000000" false false)
                      (if (Utilities|IsValid (Variables|Default|GetBP_First_FLOAT1))
                        (Actor|DestroyActor (Variables|Default|GetBP_First_FLOAT1))
                        (else
                          (Actor|DestroyActor (Variables|Default|GetBP_First_FLOAT2))))))))
              (Variables|Default|SetDo false)))
          (else
            (Development|SetHiddeninGame (Variables|Default|GetCube) false false)
            (Development|SetHiddeninGame (Variables|Default|GetCubeWidget) false false)
            (Timeline|移動まで PlayFromStart)))))))

(fn ConstructionScript)