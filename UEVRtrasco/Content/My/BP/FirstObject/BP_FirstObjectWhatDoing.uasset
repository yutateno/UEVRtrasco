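; BP_FirstObjectWhatDoing is an actor that shows one of two widgets depending on the ChangeDo state of a BP_Cube_FirstObjectProgramChange actor.
; On BeginPlay it finds all actors of that class and keeps a reference to the last one in the list.
; Every Tick it polls ChangeDo, showing Widget1 and hiding Widget when true, and the reverse when false.
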(event EventBeginPlay
  (bind _outactors (Actor|GetAllActorsOfClass "/Game/My/BP/FirstObject/BP_Cube_FirstObjectProgramChange.BP_Cube_FirstObjectProgramChange_C"))
  (for _array_element _outactors
    (Variables|Default|SetBP_Cube_FirstObjectProgramChange _array_element)))

(event Collision|EventActorBeginOverlap
  (params (OtherActor :type Actor%20Object%20Reference)))

(event EventTick
  (params (DeltaSeconds :type Float%20%28single-precision%29))
  (if (Variables|/Game/My/BP/FirstObject/BP_Cube_FirstObjectProgramChange.BP_Cube_FirstObjectProgramChange_C|GetChangeDo (Variables|Default|GetBP_Cube_FirstObjectProgramChange))
    (Development|SetHiddeninGame (Variables|Default|GetWidget) true false)
    (Development|SetHiddeninGame (Variables|Default|GetWidget1) false false)
    (else
      (Development|SetHiddeninGame (Variables|Default|GetWidget) false false)
      (Development|SetHiddeninGame (Variables|Default|GetWidget1) true false))))

(fn ConstructionScript)