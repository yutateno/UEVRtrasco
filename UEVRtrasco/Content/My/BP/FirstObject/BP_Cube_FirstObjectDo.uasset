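; BP_Cube_FirstObjectDo is a motion-controller touch cube that acts as a switch for moving BP_FirstObject.
; BeginPlay caches the BP_FirstObject found in the level, and Tick polls its MoveEnd flag to show green when touchable or dark green while it moves.
; Pickup raises the Do flag and uses a timeline as a timer to clear it, without itself checking MoveEnd.
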(event EventBeginPlay
  ;[1 1 1] BP_FirstObjectを取得して変数化する
  (bind _outactors (Actor|GetAllActorsOfClass "/Game/My/BP/FirstObject/BP_FirstObject.BP_FirstObject_C"))
  (for _array_element _outactors
    (Variables|Default|SetBP_FirstObject _array_element)))

(event Collision|EventActorBeginOverlap
  (params (OtherActor :type Actor%20Object%20Reference)))

(event EventTick
  (params (DeltaSeconds :type Float%20%28single-precision%29))
  (bind _staticmeshcomponent (Variables|Debug|GetStaticMeshComponent))
  ;[1 1 1] BP_FirstObjectが動いているかどうかで判断
  (if (Variables|/Game/My/BP/FirstObject/BP_FirstObject.BP_FirstObject_C|GetMoveEnd (Variables|Default|GetBP_FirstObject))
    ;[1 1 1] 動いていなかったらマテリアルの色を明るくして触れると分かるようにする
    (Rendering|Material|SetMaterial _staticmeshcomponent 0 "/Game/My/Material/M_Green.M_Green")
    (else
      ;[1 1 1] 動いていたらマテリアルの色を黒くして触れないと分かるようにする
      (Rendering|Material|SetMaterial _staticmeshcomponent 0 "/Game/My/Material/M_BlackGreen.M_BlackGreen"))))

(event EventPickup
  (params (AttachTo :type Scene%20Component%20Object%20Reference))
  ;[1 1 1] タッチされたらFirstCubeを動かすためのフラッグを立てて1秒で倒す
  (Variables|Default|SetDo true)
  (Timeline|タイムライン_0 Play
    (:Finished
      (Variables|Default|SetDo false))))

(event EventDrop)

(fn ConstructionScript)