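; BP_Cube_FirstObjectAdd is a VR-pickable "addition" cube that spawns new BP_Cube_FirstObjectINT actors.
; Pickup, called by BP_MotionController, increments TouchNum, spawns a quarter-scale cube at a random X on a fixed Y and Z, and stores it in an array.
; Drop is empty; detach-with-physics and clearing spawned cubes through BP_Cube_FirstObjectReset exist only as unconnected logic.
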(event EventBeginPlay)

(event Collision|EventActorBeginOverlap
  (params (OtherActor :type Actor%20Object%20Reference)))

(event EventTick
  (params (DeltaSeconds :type Float%20%28single-precision%29)))

(event EventPickup
  (params (AttachTo :type Scene%20Component%20Object%20Reference))
  ;[1 1 1] 「加算」に関する数値を増やす
  (Math|Integer|IncrementInt (Variables|Default|GetTouchNum)
    (:%20%20
      ;[1 1 1] 「加算」のアクターを動的にワールドに生成させる
      (bind _returnvalue (Game|SpawnActorfromClass "/Game/My/BP/FirstObject/BP_Cube_FirstObjectINT.BP_Cube_FirstObjectINT_C" (Math|Transform|MakeTransform (Math|Vector|MakeVector (Math|Random|RandomFloatinRange 5e+03 5.3e+03) 318.0 5e+02) "0, 0, 0" "0.250000,0.250000,0.250000") "Undefined" 0 0))
      (Utilities|Array|Add (Variables|Default|GetBP_Cube_FirstObjectINTArray) _returnvalue))))

(event EventDrop)

(fn ConstructionScript)