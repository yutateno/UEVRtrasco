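; BP_FirstObject is an actor that slides its Cube along Y as a small "program" of add and subtract steps.
; BeginPlay caches the Do, Add, Sub and ProgramChange cube actors, which Tick polls.
; A Do flag fires a DoOnce that applies Add and Sub TouchNum counts as timed MoveComponentTo moves, with ChangeDo putting subtraction first.
; Moves clamp at the far edge, or return to start when the running total drops to zero or below.
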(event EventBeginPlay
  ;[1 1 1] BP_Cube_FirstObjectDoを変数化する
  (bind _outactors (Actor|GetAllActorsOfClass "/Game/My/BP/FirstObject/BP_Cube_FirstObjectDo.BP_Cube_FirstObjectDo_C"))
  (bind _output_get (Variables|Default|SetBP_Cube_FirstObjectDoArray _outactors))
  (for _array_element _output_get
    ;[1 1 1] BP_Cube_FirstObjectAddを変数化する
    (bind _outactors_2 (Actor|GetAllActorsOfClass "/Game/My/BP/FirstObject/BP_Cube_FirstObjectAdd.BP_Cube_FirstObjectAdd_C"))
    (bind _output_get_2 (Variables|Default|SetBP_Cube_FirstObjectAddArray _outactors_2))
    (for _array_element_2 _output_get_2
      ;[1 1 1] BP_Cube_FirstObjectSubを変数化する
      (bind _outactors_3 (Actor|GetAllActorsOfClass "/Game/My/BP/FirstObject/BP_Cube_FirstObjectSub.BP_Cube_FirstObjectSub_C"))
      (bind _output_get_3 (Variables|Default|SetBP_Cube_FirstObjectSubArray _outactors_3))
      (for _array_element_3 _output_get_3
        (bind _outactors_4 (Actor|GetAllActorsOfClass "/Game/My/BP/FirstObject/BP_Cube_FirstObjectProgramChange.BP_Cube_FirstObjectProgramChange_C"))
        (bind _output_get_4 (Variables|Default|SetBP_Cube_FirstObjectProgramChangeArray _outactors_4))
        (for _array_element_4 _output_get_4
          _)))))

(event Collision|EventActorBeginOverlap
  (params (OtherActor :type Actor%20Object%20Reference)))

(event EventTick
  (params (DeltaSeconds :type Float%20%28single-precision%29))
  (bind _cube (Variables|Default|GetCube))
  (bind _cube_2 (Variables|Default|GetCube))
  (bind _cube_3 (Variables|Default|GetCube))
  (bind _cube_4 (Variables|Default|GetCube))
  (bind _cube_5 (Variables|Default|GetCube))
  (bind _cube_6 (Variables|Default|GetCube))
  (bind _returnvalue (Transformation|GetWorldLocation _cube))
  (bind _returnvalue_2 (Transformation|GetWorldLocation _cube_3))
  (bind _returnvalue_3 (Transformation|GetWorldLocation _cube_5))
  (bind _returnvalue_4 (Transformation|GetWorldLocation _cube_6))
  (for _array_element (Variables|Default|GetBP_Cube_FirstObjectProgramChangeArray)
    (if (Variables|/Game/My/BP/FirstObject/BP_Cube_FirstObjectProgramChange.BP_Cube_FirstObjectProgramChange_C|GetChangeDo _array_element)
      ;[1 1 1] 移動しているかどうか
      (if (Variables|Default|GetMoveEnd)
        ;[1 1 1] BP_Cube_FirstObjectDoの実行するフラッグが立っていたら
        (for _array_element_2 (Variables|Default|GetBP_Cube_FirstObjectDoArray)
          (if (Variables|/Game/My/BP/FirstObject/BP_Cube_FirstObjectDo.BP_Cube_FirstObjectDo_C|GetDo _array_element_2)
            (Utilities|FlowControl|DoOnce false :!label _label
              (:Completed
                ;[1 1 1] 最初のムーブが終了していないとする
                (Variables|Default|SetFirstMoveEnd false)
                ;[1 1 1] 移動中だとする
                (Variables|Default|SetMoveEnd false)
                ;[1 1 1] 「減算」の数を取得する
                (for _array_element_3 (Variables|Default|GetBP_Cube_FirstObjectSubArray)
                  ;[1 1 1] 移動した合計値に減算する
                  (bind _output_get (Variables|Default|SetNumSum (- (Variables|Default|GetNumSum) (Variables|/Game/My/BP/FirstObject/BP_Cube_FirstObjectSub.BP_Cube_FirstObjectSub_C|GetTouchNum _array_element_3))))
                  ;[1 1 1] 初期値より前に戻らされるかどうか
                  (if (> _output_get 0)
                    ;[1 1 1] 減算の個数だけ戻る
                    (Components|MoveComponentTo _cube (Math|Vector|MakeVector (.x _returnvalue) (- (.y _returnvalue) (Math|Conversions|ToFloat(Integer) (* (Variables|/Game/My/BP/FirstObject/BP_Cube_FirstObjectSub.BP_Cube_FirstObjectSub_C|GetTouchNum _array_element_3) 12))) (.z _returnvalue)) "0, 0, 0" false false 2.0 false)
                    (else
                      ;[1 1 1] 初期値まで戻る
                      (Components|MoveComponentTo _cube (Math|Vector|MakeVector (.x _returnvalue) -1619.0 (.z _returnvalue)) "0, 0, 0" false false 2.0 false)))
                  ;[1 1 1] 最初のムーブが終了したとする
                  (Variables|Default|SetFirstMoveEnd true)
                  ;[1 1 1] 「加算」の数を取得する
                  (for _array_element_4 (Variables|Default|GetBP_Cube_FirstObjectAddArray)
                    ;[1 1 1] 移動した合計値に加算する
                    (Variables|Default|SetNumSum (+ (Variables|Default|GetNumSum) (Variables|/Game/My/BP/FirstObject/BP_Cube_FirstObjectAdd.BP_Cube_FirstObjectAdd_C|GetTouchNum _array_element_4)))
                    ;[1 1 1] 端まで移動したかどうか
                    (if (>= (+ (Math|Conversions|ToFloat(Integer) (* (Variables|/Game/My/BP/FirstObject/BP_Cube_FirstObjectAdd.BP_Cube_FirstObjectAdd_C|GetTouchNum _array_element_4) 12)) (.y _returnvalue_4)) 781.0)
                      ;[1 1 1] 端まで移動していたら移動しない
                      (Components|MoveComponentTo _cube_2 (Math|Vector|MakeVector (.x _returnvalue_4) 781.0 (.z _returnvalue_4)) "0, 0, 0" false false 2.0 false)
                      (else
                        ;[1 1 1] 端まで移動していなかったら普通に移動する
                        (Components|MoveComponentTo _cube_2 (Math|Vector|MakeVector (.x _returnvalue_4) (+ (Math|Conversions|ToFloat(Integer) (* (Variables|/Game/My/BP/FirstObject/BP_Cube_FirstObjectAdd.BP_Cube_FirstObjectAdd_C|GetTouchNum _array_element_4) 12)) (.y _returnvalue_4)) (.z _returnvalue_4)) "0, 0, 0" false false 2.0 false)))
                    ;[1 1 1] 移動フラッグを倒す
                    (Variables|Default|SetMoveEnd true)))))
            (else
              (goto _label Reset)))))
      (else
        ;[1 1 1] 移動しているかどうか
        (if (Variables|Default|GetMoveEnd)
          ;[1 1 1] BP_Cube_FirstObjectDoの実行するフラッグが立っていたら
          (for _array_element_5 (Variables|Default|GetBP_Cube_FirstObjectDoArray)
            (if (Variables|/Game/My/BP/FirstObject/BP_Cube_FirstObjectDo.BP_Cube_FirstObjectDo_C|GetDo _array_element_5)
              (Utilities|FlowControl|DoOnce false :!label _label_2
                (:Completed
                  ;[1 1 1] 最初のムーブが終了していないとする
                  (Variables|Default|SetFirstMoveEnd false)
                  ;[1 1 1] 移動中だとする
                  (Variables|Default|SetMoveEnd false)
                  ;[1 1 1] 「加算」の数を取得する
                  (for _array_element_6 (Variables|Default|GetBP_Cube_FirstObjectAddArray)
                    ;[1 1 1] 移動した合計値に加算する
                    (Variables|Default|SetNumSum (+ (Variables|Default|GetNumSum) (Variables|/Game/My/BP/FirstObject/BP_Cube_FirstObjectAdd.BP_Cube_FirstObjectAdd_C|GetTouchNum _array_element_6)))
                    ;[1 1 1] 端まで移動したかどうか
                    (if (>= (+ (Math|Conversions|ToFloat(Integer) (* (Variables|/Game/My/BP/FirstObject/BP_Cube_FirstObjectAdd.BP_Cube_FirstObjectAdd_C|GetTouchNum _array_element_6) 12)) (.y _returnvalue_2)) 781.0)
                      ;[1 1 1] 端まで移動していたら移動しない
                      (Components|MoveComponentTo _cube_4 (Math|Vector|MakeVector (.x _returnvalue_2) 781.0 (.z _returnvalue_2)) "0, 0, 0" false false 2.0 false)
                      (else
                        ;[1 1 1] 端まで移動していなかったら普通に移動する
                        (Components|MoveComponentTo _cube_4 (Math|Vector|MakeVector (.x _returnvalue_2) (+ (Math|Conversions|ToFloat(Integer) (* (Variables|/Game/My/BP/FirstObject/BP_Cube_FirstObjectAdd.BP_Cube_FirstObjectAdd_C|GetTouchNum _array_element_6) 12)) (.y _returnvalue_2)) (.z _returnvalue_2)) "0, 0, 0" false false 2.0 false)))
                    ;[1 1 1] 最初のムーブが終了したとする
                    (Variables|Default|SetFirstMoveEnd true)
                    ;[1 1 1] 「減算」の数を取得する
                    (for _array_element_7 (Variables|Default|GetBP_Cube_FirstObjectSubArray)
                      ;[1 1 1] 移動した合計値に減算する
                      (bind _output_get_2 (Variables|Default|SetNumSum (- (Variables|Default|GetNumSum) (Variables|/Game/My/BP/FirstObject/BP_Cube_FirstObjectSub.BP_Cube_FirstObjectSub_C|GetTouchNum _array_element_7))))
                      ;[1 1 1] 初期値より前に戻らされるかどうか
                      (if (> _output_get_2 0)
                        ;[1 1 1] 減算の個数だけ戻る
                        (Components|MoveComponentTo _cube_5 (Math|Vector|MakeVector (.x _returnvalue_3) (- (.y _returnvalue_3) (Math|Conversions|ToFloat(Integer) (* (Variables|/Game/My/BP/FirstObject/BP_Cube_FirstObjectSub.BP_Cube_FirstObjectSub_C|GetTouchNum _array_element_7) 12))) (.z _returnvalue_3)) "0, 0, 0" false false 2.0 false)
                        (else
                          ;[1 1 1] 初期値まで戻る
                          (Components|MoveComponentTo _cube_5 (Math|Vector|MakeVector (.x _returnvalue_3) -1619.0 (.z _returnvalue_3)) "0, 0, 0" false false 2.0 false)))
                      ;[1 1 1] 移動フラッグを倒す
                      (Variables|Default|SetMoveEnd true)))))
              (else
                (goto _label_2 Reset)))))))))

(fn ConstructionScript)