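; BP_CubeBra_ProgramChange is a cube actor that switches material in response to the ChangeDo flag on a BP_Cube_FirstObjectProgramChange actor.
; BeginPlay finds actors of that class and keeps the last one as its reference.
; Tick polls the flag against a cached Touch value, and each change re-arms a DoOnce that plays a timeline setting M_Yellow on update.
; Ticks without a change apply M_BlackYellow and enter the DoOnce.
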(event EventBeginPlay
  (bind _outactors (Actor|GetAllActorsOfClass "/Game/My/BP/FirstObject/BP_Cube_FirstObjectProgramChange.BP_Cube_FirstObjectProgramChange_C"))
  (for _array_element _outactors
    (Variables|Default|SetBP_Cube_FirstObjectProgramChange _array_element)))

(event Collision|EventActorBeginOverlap
  (params (OtherActor :type Actor%20Object%20Reference)))

(event EventTick
  (params (DeltaSeconds :type Float%20%28single-precision%29))
  (bind _bp_cube_firstobjectprogramchange (Variables|Default|GetBP_Cube_FirstObjectProgramChange))
  (bind _changedo (Variables|/Game/My/BP/FirstObject/BP_Cube_FirstObjectProgramChange.BP_Cube_FirstObjectProgramChange_C|GetChangeDo _bp_cube_firstobjectprogramchange))
  (if (Math|Boolean|NotEqual(Boolean) (Variables|Default|GetTouch) _changedo)
    (Variables|Default|SetTouch _changedo)
    (goto _label Reset)
    (else
      (if _changedo
        _
        (else
          _))
      (Rendering|Material|SetMaterial (Variables|Default|GetCube) 0 "/Game/My/Material/M_BlackYellow.M_BlackYellow")
      (Utilities|FlowControl|DoOnce false :!label _label
        (:Completed
          (Timeline|タイムライン_0 PlayFromStart
            (:Update
              (Rendering|Material|SetMaterial (Variables|Default|GetCube) 0 "/Game/My/Material/M_Yellow.M_Yellow"))))))))

(fn ConstructionScript)